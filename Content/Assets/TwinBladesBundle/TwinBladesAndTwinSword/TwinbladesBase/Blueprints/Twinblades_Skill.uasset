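; Twinblades skill Blueprint that plays weapon animation montages on a skeletal mesh from hard-wired key presses, apparently as an animation showcase.
; F, G, Q and E play montages that flip SetIsTwinBlades on blend out, with IsAnimating blocking overlaps among them.
; Number keys plus second Q and E bindings trigger twelve attack montages without that guard.
; K plays all twelve in sequence through nested Blend Out callbacks.
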(event EventBeginPlay)

(event Collision|EventActorBeginOverlap
  (params (OtherActor :type Actor%20Object%20Reference)))

(event EventTick
  (params (DeltaSeconds :type Float%20%28single-precision%29)))

(event Input|KeyboardEvents|F
  (params (Key :type Key%20Structure))
  (:Pressed
    (if (not (Variables|Default|GetIsAnimating))
      (Variables|Default|SetIsAnimating true)
      (if (Variables|Default|GetSet%20IsTwinBlades)
        (Animation|Montage|PlayMontage (Variables|Character|GetMesh) 0
          (:OnBlendOut
            (Variables|Default|SetSet%20IsTwinBlades false)
            (Variables|Default|SetIsAnimating false)))
        (else
          (Animation|Montage|PlayMontage (Variables|Character|GetMesh) 0
            (:OnBlendOut
              (Variables|Default|SetSet%20IsTwinBlades true)
              (Variables|Default|SetIsAnimating false))))))))

(event Input|KeyboardEvents|1
  (params (Key :type Key%20Structure))
  (:Pressed
    (Animation|Montage|PlayMontage (Variables|Character|GetMesh) "/Game/Assets/TwinBladesBundle/TwinBladesAndTwinSword/TwinbladesBase/Animation/Attack/Twinblades_Attack_01_Montage.Twinblades_Attack_01_Montage")))

(event Input|KeyboardEvents|2
  (params (Key :type Key%20Structure))
  (:Pressed
    (Animation|Montage|PlayMontage (Variables|Character|GetMesh) "/Game/Assets/TwinBladesBundle/TwinBladesAndTwinSword/TwinbladesBase/Animation/Attack/Twinblades_Attack_02_Montage.Twinblades_Attack_02_Montage")))

(event Input|KeyboardEvents|3
  (params (Key :type Key%20Structure))
  (:Pressed
    (Animation|Montage|PlayMontage (Variables|Character|GetMesh) "/Game/Assets/TwinBladesBundle/TwinBladesAndTwinSword/TwinbladesBase/Animation/Attack/Twinblades_Attack_03_Montage.Twinblades_Attack_03_Montage")))

(event Input|KeyboardEvents|4
  (params (Key :type Key%20Structure))
  (:Pressed
    (Animation|Montage|PlayMontage (Variables|Character|GetMesh) "/Game/Assets/TwinBladesBundle/TwinBladesAndTwinSword/TwinbladesBase/Animation/Attack/Twinblades_Attack_04_Montage.Twinblades_Attack_04_Montage")))

(event Input|KeyboardEvents|G
  (params (Key :type Key%20Structure))
  (:Pressed
    (if (not (Variables|Default|GetIsAnimating))
      (Variables|Default|SetIsAnimating true)
      (if (Variables|Default|GetSet%20IsTwinBlades)
        (Animation|Montage|PlayMontage (Variables|Character|GetMesh) 0
          (:OnBlendOut
            (Variables|Default|SetSet%20IsTwinBlades false)
            (Variables|Default|SetIsAnimating false)))
        (else
          (Animation|Montage|PlayMontage (Variables|Character|GetMesh) 0
            (:OnBlendOut
              (Variables|Default|SetSet%20IsTwinBlades true)
              (Variables|Default|SetIsAnimating false))))))))

(event Input|KeyboardEvents|5
  (params (Key :type Key%20Structure))
  (:Pressed
    (Animation|Montage|PlayMontage (Variables|Character|GetMesh) "/Game/Assets/TwinBladesBundle/TwinBladesAndTwinSword/TwinbladesBase/Animation/Attack/Twinblades_Attack_05_Montage.Twinblades_Attack_05_Montage")))

(event Input|KeyboardEvents|6
  (params (Key :type Key%20Structure))
  (:Pressed
    (Animation|Montage|PlayMontage (Variables|Character|GetMesh) "/Game/Assets/TwinBladesBundle/TwinBladesAndTwinSword/TwinbladesBase/Animation/Attack/Twinblades_Attack_06_Montage.Twinblades_Attack_06_Montage")))

(event Input|KeyboardEvents|7
  (params (Key :type Key%20Structure))
  (:Pressed
    (Animation|Montage|PlayMontage (Variables|Character|GetMesh) "/Game/Assets/TwinBladesBundle/TwinBladesAndTwinSword/TwinbladesBase/Animation/Attack/Twinblades_Attack_07_Montage.Twinblades_Attack_07_Montage")))

(event Input|KeyboardEvents|8
  (params (Key :type Key%20Structure))
  (:Pressed
    (Animation|Montage|PlayMontage (Variables|Character|GetMesh) "/Game/Assets/TwinBladesBundle/TwinBladesAndTwinSword/TwinbladesBase/Animation/Attack/Twinblades_Attack_08_Montage.Twinblades_Attack_08_Montage")))

(event Input|KeyboardEvents|9
  (params (Key :type Key%20Structure))
  (:Pressed
    (Animation|Montage|PlayMontage (Variables|Character|GetMesh) "/Game/Assets/TwinBladesBundle/TwinBladesAndTwinSword/TwinbladesBase/Animation/Attack/Twinblades_Attack_09_Montage.Twinblades_Attack_09_Montage")))

(event Input|KeyboardEvents|0
  (params (Key :type Key%20Structure))
  (:Pressed
    (Animation|Montage|PlayMontage (Variables|Character|GetMesh) "/Game/Assets/TwinBladesBundle/TwinBladesAndTwinSword/TwinbladesBase/Animation/Attack/Twinblades_Attack_10_Montage.Twinblades_Attack_10_Montage")))

(event Input|KeyboardEvents|Q
  (params (Key :type Key%20Structure))
  (:Pressed
    (Animation|Montage|PlayMontage (Variables|Character|GetMesh) "/Game/Assets/TwinBladesBundle/TwinBladesAndTwinSword/TwinbladesBase/Animation/Attack/Twinblades_Attack_11_Montage.Twinblades_Attack_11_Montage")))

(event Input|KeyboardEvents|E
  (params (Key :type Key%20Structure))
  (:Pressed
    (Animation|Montage|PlayMontage (Variables|Character|GetMesh) "/Game/Assets/TwinBladesBundle/TwinBladesAndTwinSword/TwinbladesBase/Animation/Attack/Twinblades_Attack_12_Montage.Twinblades_Attack_12_Montage")))

(event Input|KeyboardEvents|Q
  (params (Key :type Key%20Structure))
  (:Pressed
    (if (not (Variables|Default|GetIsAnimating))
      (Variables|Default|SetIsAnimating true)
      (if (Variables|Default|GetSet%20IsTwinBlades)
        (Animation|Montage|PlayMontage (Variables|Character|GetMesh) 0
          (:OnBlendOut
            (Variables|Default|SetSet%20IsTwinBlades false)
            (Variables|Default|SetIsAnimating false)))
        (else
          (Animation|Montage|PlayMontage (Variables|Character|GetMesh) 0
            (:OnBlendOut
              (Variables|Default|SetSet%20IsTwinBlades true)
              (Variables|Default|SetIsAnimating false))))))))

(event Input|KeyboardEvents|E
  (params (Key :type Key%20Structure))
  (:Pressed
    (if (not (Variables|Default|GetIsAnimating))
      (Variables|Default|SetIsAnimating true)
      (if (Variables|Default|GetSet%20IsTwinBlades)
        (Animation|Montage|PlayMontage (Variables|Character|GetMesh) 0
          (:OnBlendOut
            (Variables|Default|SetSet%20IsTwinBlades false)
            (Variables|Default|SetIsAnimating false)))
        (else
          (Animation|Montage|PlayMontage (Variables|Character|GetMesh) 0
            (:OnBlendOut
              (Variables|Default|SetSet%20IsTwinBlades true)
              (Variables|Default|SetIsAnimating false))))))))

(event Input|KeyboardEvents|K
  (params (Key :type Key%20Structure))
  (:Pressed
    (Animation|Montage|PlayMontage (Variables|Character|GetMesh) "/Game/Assets/TwinBladesBundle/TwinBladesAndTwinSword/TwinbladesBase/Animation/Attack/Twinblades_Attack_01_Montage.Twinblades_Attack_01_Montage"
      (:OnBlendOut
        (Animation|Montage|PlayMontage (Variables|Character|GetMesh) "/Game/Assets/TwinBladesBundle/TwinBladesAndTwinSword/TwinbladesBase/Animation/Attack/Twinblades_Attack_02_Montage.Twinblades_Attack_02_Montage"
          (:OnBlendOut
            (Animation|Montage|PlayMontage (Variables|Character|GetMesh) "/Game/Assets/TwinBladesBundle/TwinBladesAndTwinSword/TwinbladesBase/Animation/Attack/Twinblades_Attack_03_Montage.Twinblades_Attack_03_Montage"
              (:OnBlendOut
                (Animation|Montage|PlayMontage (Variables|Character|GetMesh) "/Game/Assets/TwinBladesBundle/TwinBladesAndTwinSword/TwinbladesBase/Animation/Attack/Twinblades_Attack_04_Montage.Twinblades_Attack_04_Montage"
                  (:OnBlendOut
                    (Animation|Montage|PlayMontage (Variables|Character|GetMesh) "/Game/Assets/TwinBladesBundle/TwinBladesAndTwinSword/TwinbladesBase/Animation/Attack/Twinblades_Attack_05_Montage.Twinblades_Attack_05_Montage"
                      (:OnBlendOut
                        (Animation|Montage|PlayMontage (Variables|Character|GetMesh) "/Game/Assets/TwinBladesBundle/TwinBladesAndTwinSword/TwinbladesBase/Animation/Attack/Twinblades_Attack_06_Montage.Twinblades_Attack_06_Montage"
                          (:OnBlendOut
                            (Animation|Montage|PlayMontage (Variables|Character|GetMesh) "/Game/Assets/TwinBladesBundle/TwinBladesAndTwinSword/TwinbladesBase/Animation/Attack/Twinblades_Attack_07_Montage.Twinblades_Attack_07_Montage"
                              (:OnBlendOut
                                (Animation|Montage|PlayMontage (Variables|Character|GetMesh) "/Game/Assets/TwinBladesBundle/TwinBladesAndTwinSword/TwinbladesBase/Animation/Attack/Twinblades_Attack_08_Montage.Twinblades_Attack_08_Montage"
                                  (:OnBlendOut
                                    (Animation|Montage|PlayMontage (Variables|Character|GetMesh) "/Game/Assets/TwinBladesBundle/TwinBladesAndTwinSword/TwinbladesBase/Animation/Attack/Twinblades_Attack_09_Montage.Twinblades_Attack_09_Montage"
                                      (:OnBlendOut
                                        (Animation|Montage|PlayMontage (Variables|Character|GetMesh) "/Game/Assets/TwinBladesBundle/TwinBladesAndTwinSword/TwinbladesBase/Animation/Attack/Twinblades_Attack_10_Montage.Twinblades_Attack_10_Montage"
                                          (:OnBlendOut
                                            (Animation|Montage|PlayMontage (Variables|Character|GetMesh) "/Game/Assets/TwinBladesBundle/TwinBladesAndTwinSword/TwinbladesBase/Animation/Attack/Twinblades_Attack_11_Montage.Twinblades_Attack_11_Montage"
                                              (:OnBlendOut
                                                (Animation|Montage|PlayMontage (Variables|Character|GetMesh) "/Game/Assets/TwinBladesBundle/TwinBladesAndTwinSword/TwinbladesBase/Animation/Attack/Twinblades_Attack_12_Montage.Twinblades_Attack_12_Montage")))))))))))))))))))))))))

(fn ConstructionScript)