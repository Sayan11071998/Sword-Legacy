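; Demo character Blueprint that previews twinblade attack montages from keyboard input on its mesh.
; Number keys each play a single montage, mostly from the Attack13 to Attack20 set, though key 0 has none assigned.
; K plays the attacks as a sequence chained through Blend Out, ending in three plays with no montage assigned.
; Disconnected leftover graphs hold an unused twinblade stance toggle guarded by IsAnimating.
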(event EventBeginPlay)

(event Collision|EventActorBeginOverlap
  (params (OtherActor :type Actor%20Object%20Reference)))

(event EventTick
  (params (DeltaSeconds :type Float%20%28single-precision%29)))

(event Input|KeyboardEvents|F
  (params (Key :type Key%20Structure)))

(event Input|KeyboardEvents|1
  (params (Key :type Key%20Structure))
  (:Pressed
    (Animation|Montage|PlayMontage (Variables|Character|GetMesh) "/Game/Assets/TwinBladesBundle/TwinBladesAndTwinSword/TwinbladesExpansion/Animation/Attack/Twinblades_Attack13_Montage.Twinblades_Attack13_Montage")))

(event Input|KeyboardEvents|2
  (params (Key :type Key%20Structure))
  (:Pressed
    (Animation|Montage|PlayMontage (Variables|Character|GetMesh) "/Game/Assets/TwinBladesBundle/TwinBladesAndTwinSword/TwinbladesExpansion/Animation/Attack/Twinblades_Attack14_Montage.Twinblades_Attack14_Montage")))

(event Input|KeyboardEvents|3
  (params (Key :type Key%20Structure))
  (:Pressed
    (Animation|Montage|PlayMontage (Variables|Character|GetMesh) "/Game/Assets/TwinBladesBundle/TwinBladesAndTwinSword/TwinbladesExpansion/Animation/Attack/Twinblades_Attack15_Montage.Twinblades_Attack15_Montage")))

(event Input|KeyboardEvents|4
  (params (Key :type Key%20Structure))
  (:Pressed
    (Animation|Montage|PlayMontage (Variables|Character|GetMesh) "/Game/Assets/TwinBladesBundle/TwinBladesAndTwinSword/TwinbladesExpansion/Animation/Attack/Twinblades_Attack16_Montage.Twinblades_Attack16_Montage")))

(event Input|KeyboardEvents|G
  (params (Key :type Key%20Structure)))

(event Input|KeyboardEvents|5
  (params (Key :type Key%20Structure))
  (:Pressed
    (Animation|Montage|PlayMontage (Variables|Character|GetMesh) "/Game/Assets/TwinBladesBundle/TwinBladesAndTwinSword/TwinbladesExpansion/Animation/Attack/Twinblades_Attack17_1_Montage.Twinblades_Attack17_1_Montage")))

(event Input|KeyboardEvents|6
  (params (Key :type Key%20Structure))
  (:Pressed
    (Animation|Montage|PlayMontage (Variables|Character|GetMesh) "/Game/Assets/TwinBladesBundle/TwinBladesAndTwinSword/TwinbladesExpansion/Animation/Attack/Twinblades_Attack17_Montage.Twinblades_Attack17_Montage")))

(event Input|KeyboardEvents|7
  (params (Key :type Key%20Structure))
  (:Pressed
    (Animation|Montage|PlayMontage (Variables|Character|GetMesh) "/Game/Assets/TwinBladesBundle/TwinBladesAndTwinSword/TwinbladesExpansion/Animation/Attack/Twinblades_Attack18_Montage.Twinblades_Attack18_Montage")))

(event Input|KeyboardEvents|8
  (params (Key :type Key%20Structure))
  (:Pressed
    (Animation|Montage|PlayMontage (Variables|Character|GetMesh) "/Game/Assets/TwinBladesBundle/TwinBladesAndTwinSword/TwinbladesExpansion/Animation/Attack/Twinblades_Attack19_Montage.Twinblades_Attack19_Montage")))

(event Input|KeyboardEvents|9
  (params (Key :type Key%20Structure))
  (:Pressed
    (Animation|Montage|PlayMontage (Variables|Character|GetMesh) "/Game/Assets/TwinBladesBundle/TwinBladesAndTwinSword/TwinbladesExpansion/Animation/Attack/Twinblades_Attack20_Montage.Twinblades_Attack20_Montage")))

(event Input|KeyboardEvents|0
  (params (Key :type Key%20Structure))
  (:Pressed
    (Animation|Montage|PlayMontage (Variables|Character|GetMesh) 0)))

(event Input|KeyboardEvents|Q
  (params (Key :type Key%20Structure)))

(event Input|KeyboardEvents|E
  (params (Key :type Key%20Structure)))

(event Input|KeyboardEvents|Q
  (params (Key :type Key%20Structure)))

(event Input|KeyboardEvents|E
  (params (Key :type Key%20Structure)))

(event Input|KeyboardEvents|K
  (params (Key :type Key%20Structure))
  (:Pressed
    (Animation|Montage|PlayMontage (Variables|Character|GetMesh) "/Game/Assets/TwinBladesBundle/TwinBladesAndTwinSword/TwinbladesExpansion/Animation/Attack/Twinblades_Attack13_Montage.Twinblades_Attack13_Montage"
      (:OnBlendOut
        (Animation|Montage|PlayMontage (Variables|Character|GetMesh) "/Game/Assets/TwinBladesBundle/TwinBladesAndTwinSword/TwinbladesExpansion/Animation/Attack/Twinblades_Attack14_Montage.Twinblades_Attack14_Montage"
          (:OnBlendOut
            (Animation|Montage|PlayMontage (Variables|Character|GetMesh) "/Game/Assets/TwinBladesBundle/TwinBladesAndTwinSword/TwinbladesExpansion/Animation/Attack/Twinblades_Attack15_Montage.Twinblades_Attack15_Montage"
              (:OnBlendOut
                (Animation|Montage|PlayMontage (Variables|Character|GetMesh) "/Game/Assets/TwinBladesBundle/TwinBladesAndTwinSword/TwinbladesExpansion/Animation/Attack/Twinblades_Attack16_Montage.Twinblades_Attack16_Montage"
                  (:OnBlendOut
                    (Animation|Montage|PlayMontage (Variables|Character|GetMesh) "/Game/Assets/TwinBladesBundle/TwinBladesAndTwinSword/TwinbladesExpansion/Animation/Attack/Twinblades_Attack17_1_Montage.Twinblades_Attack17_1_Montage"
                      (:OnBlendOut
                        (Animation|Montage|PlayMontage (Variables|Character|GetMesh) "/Game/Assets/TwinBladesBundle/TwinBladesAndTwinSword/TwinbladesExpansion/Animation/Attack/Twinblades_Attack18_Montage.Twinblades_Attack18_Montage"
                          (:OnBlendOut
                            (Animation|Montage|PlayMontage (Variables|Character|GetMesh) "/Game/Assets/TwinBladesBundle/TwinBladesAndTwinSword/TwinbladesExpansion/Animation/Attack/Twinblades_Attack19_Montage.Twinblades_Attack19_Montage"
                              (:OnBlendOut
                                (Animation|Montage|PlayMontage (Variables|Character|GetMesh) "/Game/Assets/TwinBladesBundle/TwinBladesAndTwinSword/TwinbladesExpansion/Animation/Attack/Twinblades_Attack20_Montage.Twinblades_Attack20_Montage"
                                  (:OnBlendOut
                                    (Animation|Montage|PlayMontage (Variables|Character|GetMesh) 0
                                      (:OnBlendOut
                                        (Animation|Montage|PlayMontage (Variables|Character|GetMesh) 0
                                          (:OnBlendOut
                                            (Animation|Montage|PlayMontage (Variables|Character|GetMesh) 0)))))))))))))))))))))))

(fn ConstructionScript)