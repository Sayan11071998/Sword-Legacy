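; Player controller Blueprint whose BeginPlay is empty, leaving its frontend UI and input setup disconnected so it never runs.
; The unwired chain creates the primary layout widget, registers it with the SLUI subsystem, then pushes the tag-resolved Press Any Key screen onto the Frontend widget stack.
; A second sequence branch registers the default mapping context with Enhanced Input user settings.
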(event EventBeginPlay)

(fn ConstructionScript)