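; Base enemy character Blueprint holding a death dissolve sequence, though no event in its graph triggers it.
; The sequence pauses animation, disables capsule collision, clears enemy UI widgets and async-loads a Niagara effect.
; The effect takes its color from the mesh material's dissolve edge color.
; A duration-scaled timeline drives DissolveAmount on mesh and equipped weapon, then destroys both actors.
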(fn ConstructionScript)